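; BP_ShaderActor is a test actor that drives a custom shader drawing into the ShaderTestRT render target.
; On BeginPlay it clears the target, then calls DrawTestShaderRenderTarget with a color, the T_RhodesIsland texture and a struct of four preset colors plus ColorIndex.
; Keys 1 to 4 set ColorIndex and redraw, so rendering happens only at startup and on key press.
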(event EventBeginPlay
  (Rendering|ClearRenderTarget2D "/Game/CustomShader/ShaderTestRT.ShaderTestRT" "(R=1.000000,G=0.000000,B=0.794383,A=1.000000)")
  (Class|TestShaderBlueprintLibrary|DrawTestShaderRenderTarget "/Game/CustomShader/ShaderTestRT.ShaderTestRT" self (Variables|Default|GetColor) "/Game/CustomShader/T_RhodesIsland.T_RhodesIsland" (Utilities|Struct|MakeMyShaderStructData "(R=1.000000,G=0.000000,B=0.369439,A=1.000000)" "(R=0.000000,G=1.000000,B=1.000000,A=1.000000)" "(R=0.800698,G=0.984375,B=0.079646,A=1.000000)" "(R=0.000000,G=0.116427,B=0.800000,A=1.000000)" (Variables|Default|GetColorIndex))))

(event Input|KeyboardEvents|1
  (params (Key :type Key%20Structure :default "None"))
  (:Pressed
    (Variables|Default|SetColorIndex 0)
    (Class|TestShaderBlueprintLibrary|DrawTestShaderRenderTarget "/Game/CustomShader/ShaderTestRT.ShaderTestRT" self (Variables|Default|GetColor) "/Game/CustomShader/T_RhodesIsland.T_RhodesIsland" (Utilities|Struct|MakeMyShaderStructData "(R=1.000000,G=0.000000,B=0.369439,A=1.000000)" "(R=0.000000,G=1.000000,B=1.000000,A=1.000000)" "(R=0.800698,G=0.984375,B=0.079646,A=1.000000)" "(R=0.000000,G=0.116427,B=0.800000,A=1.000000)" (Variables|Default|GetColorIndex)))))

(event Input|KeyboardEvents|2
  (params (Key :type Key%20Structure :default "None"))
  (:Pressed
    (Variables|Default|SetColorIndex 1)
    (Class|TestShaderBlueprintLibrary|DrawTestShaderRenderTarget "/Game/CustomShader/ShaderTestRT.ShaderTestRT" self (Variables|Default|GetColor) "/Game/CustomShader/T_RhodesIsland.T_RhodesIsland" (Utilities|Struct|MakeMyShaderStructData "(R=1.000000,G=0.000000,B=0.369439,A=1.000000)" "(R=0.000000,G=1.000000,B=1.000000,A=1.000000)" "(R=0.800698,G=0.984375,B=0.079646,A=1.000000)" "(R=0.000000,G=0.116427,B=0.800000,A=1.000000)" (Variables|Default|GetColorIndex)))))

(event Input|KeyboardEvents|3
  (params (Key :type Key%20Structure :default "None"))
  (:Pressed
    (Variables|Default|SetColorIndex 2)
    (Class|TestShaderBlueprintLibrary|DrawTestShaderRenderTarget "/Game/CustomShader/ShaderTestRT.ShaderTestRT" self (Variables|Default|GetColor) "/Game/CustomShader/T_RhodesIsland.T_RhodesIsland" (Utilities|Struct|MakeMyShaderStructData "(R=1.000000,G=0.000000,B=0.369439,A=1.000000)" "(R=0.000000,G=1.000000,B=1.000000,A=1.000000)" "(R=0.800698,G=0.984375,B=0.079646,A=1.000000)" "(R=0.000000,G=0.116427,B=0.800000,A=1.000000)" (Variables|Default|GetColorIndex)))))

(event Input|KeyboardEvents|4
  (params (Key :type Key%20Structure :default "None"))
  (:Pressed
    (Variables|Default|SetColorIndex 3)
    (Class|TestShaderBlueprintLibrary|DrawTestShaderRenderTarget "/Game/CustomShader/ShaderTestRT.ShaderTestRT" self (Variables|Default|GetColor) "/Game/CustomShader/T_RhodesIsland.T_RhodesIsland" (Utilities|Struct|MakeMyShaderStructData "(R=1.000000,G=0.000000,B=0.369439,A=1.000000)" "(R=0.000000,G=1.000000,B=1.000000,A=1.000000)" "(R=0.800698,G=0.984375,B=0.079646,A=1.000000)" "(R=0.000000,G=0.116427,B=0.800000,A=1.000000)" (Variables|Default|GetColorIndex)))))

(fn ConstructionScript)